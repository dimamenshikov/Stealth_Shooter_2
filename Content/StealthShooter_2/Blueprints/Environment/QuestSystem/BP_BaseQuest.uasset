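; Base quest Blueprint for the stealth shooter that builds and displays a quest's UI and reports its outcome.
; On BeginPlay it creates a quest widget from its name and number, then fills it with one numbered task widget per task entry.
; Start adds that widget to the viewport.
; WinDefeat sets the result text and color on the quest system widget and plays an optional sound at the game options volume.
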(event Custom|Start
  ;[0 0 0] Создание виджета квеста, его имени, номера, добавление задач, вывод на экран при старте квеста
  (UserInterface|Viewport|AddtoViewport (Variables|Default|GetWidgetQuest) 0))

(event EventBeginPlay
  ;[0 0 0] Создание виджета квеста, его имени, номера, добавление задач, вывод на экран при старте квеста
  (bind _returnvalue (UserInterface|CreateWidget "/Game/StealthShooter_2/Widgets/WBP_Quest.WBP_Quest_C" 0 (Variables|Default|GetName) (Variables|Default|GetNumber)))
  (bind _output_get (Variables|Default|SetWidgetQuest _returnvalue))
  (for (_array_element _array_index) (Variables|Default|GetTask)
    (bind _returnvalue_2 (UserInterface|CreateWidget "/Game/StealthShooter_2/Widgets/WBP_TaskQuest.WBP_TaskQuest_C" 0 _array_element (+ _array_index 1)))
    (Utilities|Array|Add (Variables|Default|GetTasks) _returnvalue_2)
    (Widget|Panel|AddChild (Variables|/Game/StealthShooter_2/Widgets/WBP_Quest.WBP_Quest_C|GetTasks _output_get) _returnvalue_2)))

(fn ConstructionScript)

(fn WinDefeat
  (params (Result :type Text) (InColorAndOpacity :type Slate%20Color%20Structure) (Sound :type Sound%20Base%20Object%20Reference))
  (bind _questwidgetsystem (Variables|Default|GetQuestWidgetSystem))
  (bind _resultquest (Variables|/Game/StealthShooter_2/Widgets/WBP_Quests.WBP_Quests_C|GetResultQuest _questwidgetsystem))
  ;[0 0 0] Вывод результата квеста, проигрывание звука
  (Variables|/Script/UMG.TextBlock|SetText _resultquest Result)
  (Appearance|SetColorandOpacity _resultquest InColorAndOpacity :!class /Script/UMG.TextBlock)
  (Utilities|IsValid Sound
    (:Is%20Valid
      (Audio|PlaySound2D Sound (.volume (Variables|/Game/StealthShooter_2/Blueprints/Core/BP_GameInstance.BP_GameInstance_C|GetGameOptions (CallFunction|GameInstance))) 1.0 0.0 0 0))
    (:Is%20Not%20Valid
      _))
  (return))