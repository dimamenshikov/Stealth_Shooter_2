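; Level quest manager that runs BP_BaseQuest actors sequentially in ascending Number order and handles win or loss.
; On BeginPlay it gathers and sorts the quests into a map and shares one WBP_Quests widget with them.
; GameInstance's start event shows the widget and starts the first quest; each OnComplete success advances the chain, ending the game on LastLevel.
; Failure can cost a life, then reloads the level or ends the game at zero lives.
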(event Custom|StartGame
  ;[0 0 0] Создание виджета для квестов, получение ссылок всех квестов на уровне, запуск первого квеста
  (UserInterface|Viewport|AddtoViewport (Variables|Default|GetQuestWidget) 0)
  (CallFunction|StartNewQuest))

(event Custom|StartNewQuest
  (bind _quests (Variables|Default|GetQuests))
  (bind _currentquest (Variables|Default|GetCurrentQuest))
  (bind (_value _returnvalue) (Utilities|Map|Find _quests _currentquest))
  ;[0 0 0] Старт слудеющего квеста, подписка на его результат, конец игры
  (if _returnvalue
    (EventDispatchers|BindEventtoOnComplete _value (delegate Custom|Complete))
    (Widget|Panel|AddChild (Variables|/Game/StealthShooter_2/Widgets/WBP_Quests.WBP_Quests_C|GetQuests (Variables|Default|GetQuestWidget)) (Variables|/Game/StealthShooter_2/Blueprints/Environment/QuestSystem/BP_BaseQuest.BP_BaseQuest_C|GetWidgetQuest _value))
    (Default|Start _value)))

(event Custom|Complete
  (params (Success :type Boolean) (Quest :type BP%20Base%20Quest%20Object%20Reference))
  (bind _gameplayclasses (Variables|Default|GetGameplayClasses))
  (bind _gameplayclasses_2 (Variables|Default|GetGameplayClasses))
  (bind _playercharacter (Variables|/Game/StealthShooter_2/Blueprints/DataAsset/PDA_GameplayClasses.PDA_GameplayClasses_C|GetPlayerCharacter _gameplayclasses_2))
  (bind _life (Variables|/Game/StealthShooter_2/Blueprints/Core/Character/BP_BaseCharacter.BP_BaseCharacter_C|GetLife _playercharacter))
  ;[0 0 0] Старт слудеющего квеста, подписка на его результат, конец игры
  (EventDispatchers|UnbindallEventsfromOnComplete Quest)
  (if Success
    (bind _result (Math|Integer|IncrementInt (Variables|Default|GetCurrentQuest))
      (:%20%20
        (if (.ReturnValue (Utilities|Map|Find (Variables|Default|GetQuests) _result))
          (CallFunction|StartNewQuest)
          (elif (Variables|Default|GetbLastLevel)
            (Utilities|FlowControl|Delay 2.0)
            (Default|EndGame (Variables|/Game/StealthShooter_2/Blueprints/DataAsset/PDA_GameplayClasses.PDA_GameplayClasses_C|GetGameMode (Variables|Default|GetGameplayClasses)) true)))))
    (else
      (if (== 0.0 (Variables|/Game/StealthShooter_2/Blueprints/Core/Character/BP_BaseCharacter.BP_BaseCharacter_C|GetHealth _playercharacter))
        _
        (else
          (Math|Integer|DecrementInt _life
            (:%20%20
              _))))
      (if (== _life 0)
        (Default|EndGame (Variables|/Game/StealthShooter_2/Blueprints/DataAsset/PDA_GameplayClasses.PDA_GameplayClasses_C|GetGameMode (Variables|Default|GetGameplayClasses)) false)
        (else
          (Utilities|FlowControl|Delay 3.0)
          (Variables|/Game/StealthShooter_2/Blueprints/Core/BP_GameInstance.BP_GameInstance_C|SetPlayerLife (Variables|/Game/StealthShooter_2/Blueprints/DataAsset/PDA_GameplayClasses.PDA_GameplayClasses_C|GetGameInstance _gameplayclasses) (Variables|/Game/StealthShooter_2/Blueprints/Core/Character/BP_BaseCharacter.BP_BaseCharacter_C|GetLife (Variables|/Game/StealthShooter_2/Blueprints/DataAsset/PDA_GameplayClasses.PDA_GameplayClasses_C|GetPlayerCharacter _gameplayclasses)))
          (bind _returnvalue (Game|GetCurrentLevelName true))
          (Game|OpenLevel(byName) (Utilities|String|StringToName _returnvalue)))))))

(event EventBeginPlay
  (bind _tempmap (Variables|Default|GetTempMap))
  ;[0 0 0] Создание виджета для квестов, получение ссылок всех квестов на уровне, запуск первого квеста
  (EventDispatchers|BindEventtoOnStartGame (Variables|/Game/StealthShooter_2/Blueprints/DataAsset/PDA_GameplayClasses.PDA_GameplayClasses_C|GetGameInstance (Variables|Default|GetGameplayClasses)) (delegate Custom|StartGame))
  (bind _returnvalue (UserInterface|CreateWidget "/Game/StealthShooter_2/Widgets/WBP_Quests.WBP_Quests_C"))
  (Variables|Default|SetQuestWidget _returnvalue)
  (bind _outactors (Actor|GetAllActorsOfClass "/Game/StealthShooter_2/Blueprints/Environment/QuestSystem/BP_BaseQuest.BP_BaseQuest_C"))
  (for _array_element _outactors
    (Utilities|Map|Add (Variables|Default|GetTempMap) (Variables|/Game/StealthShooter_2/Blueprints/Environment/QuestSystem/BP_BaseQuest.BP_BaseQuest_C|GetNumber _array_element) _array_element)
    (Variables|/Game/StealthShooter_2/Blueprints/Environment/QuestSystem/BP_BaseQuest.BP_BaseQuest_C|SetQuestWidgetSystem _array_element (Variables|Default|GetQuestWidget)))
  (bind _keys (Utilities|Map|Keys _tempmap))
  (Variables|Default|SetCurrentQuest (.MinValue (Math|Integer|MinOfIntArray _keys)))
  (while (Utilities|Array|IsNotEmpty _keys)
    (Utilities|Map|Add (Variables|Default|GetQuests) (.MinValue (Math|Integer|MinOfIntArray _keys)) (.Value (Utilities|Map|Find _tempmap (.MinValue (Math|Integer|MinOfIntArray _keys)))))
    (Utilities|Array|RemoveIndex _keys (.IndexOfMinValue (Math|Integer|MinOfIntArray _keys)))))

(fn ConstructionScript)