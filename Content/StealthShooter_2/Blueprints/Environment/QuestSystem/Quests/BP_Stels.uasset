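; BP_Stels is a stealth quest in which the player must collect ammo without being detected by enemies.
; Start runs a gated per-tick loop over all AIC_Enemy controllers, failing the quest when a blackboard reports PlayerDetected.
; Box1 overlap adds the take-ammo task to the quest widget once.
; Box overlap with enough ammo closes the gate, shows victory, completes the quest, saves player data and opens a level.
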(event OnComponentBeginOverlap(Box)
  (params (OverlappedComponent :type Primitive%20Component%20Object%20Reference) (OtherActor :type Actor%20Object%20Reference) (OtherComp :type Primitive%20Component%20Object%20Reference) (OtherBodyIndex :type Integer) (bFromSweep :type Boolean) (SweepResult :type Hit%20Result%20Structure%20%28by%20ref%29))
  (bind _asbp_player_character_stealth_shooter_2 (Utilities|Casting|CastToBP_PlayerCharacterStealthShooter_2 OtherActor))
  (if (>= (Variables|/Game/StealthShooter_2/Blueprints/Core/Character/BP_BaseCharacter.BP_BaseCharacter_C|GetPatronsInEquipment _asbp_player_character_stealth_shooter_2) 60)
    (Utilities|FlowControl|Sequence
      (:then_0
        (CallFunction|WinDefeat "Миссия выполнена!" (Utilities|Struct|MakeSlateColor "(R=0.000000,G=0.500000,B=0.000000,A=1.000000)" "UseColor_Specified") "/Game/StealthShooter_2/Assets/Sound/A_Win.A_Win")
        (Default|CallOnComplete true self)
        (Default|SaveDataPlayer (Variables|/Game/StealthShooter_2/Blueprints/DataAsset/PDA_GameplayClasses.PDA_GameplayClasses_C|GetGameInstance (Variables|Default|GetGameplayClasses)))
        (Utilities|FlowControl|Delay 1.0)
        (Game|OpenLevel(byObjectReference) (Variables|Default|GetLevel)))
      (:then_1
        (Utilities|FlowControl|Gate false) ; enters at Close
      ))))

(event OnComponentBeginOverlap(Box1)
  (params (OverlappedComponent :type Primitive%20Component%20Object%20Reference) (OtherActor :type Actor%20Object%20Reference) (OtherComp :type Primitive%20Component%20Object%20Reference) (OtherBodyIndex :type Integer) (bFromSweep :type Boolean) (SweepResult :type Hit%20Result%20Structure%20%28by%20ref%29))
  (Utilities|FlowControl|DoOnce false
    (:Completed
      (Class|BPIActivate|Activate(Message) (Variables|Default|GetActor) false)
      (bind _returnvalue (Utilities|Array|Add (Variables|Default|GetTask) "Взять патроны"))
      (bind _returnvalue_2 (UserInterface|CreateWidget "/Game/StealthShooter_2/Widgets/WBP_TaskQuest.WBP_TaskQuest_C" 0 "Взять патроны" (+ _returnvalue 1)))
      (Utilities|Array|Add (Variables|Default|GetTasks) _returnvalue_2)
      (Widget|Panel|AddChild (Variables|/Game/StealthShooter_2/Widgets/WBP_Quest.WBP_Quest_C|GetTasks (Variables|Default|GetWidgetQuest)) _returnvalue_2))))

(event EventStart
  (bind _outactors (Actor|GetAllActorsOfClass "/Game/StealthShooter_2/AI/Guard/AIC_Enemy.AIC_Enemy_C" :!label _label))
  (if (Utilities|Array|IsNotEmpty _outactors)
    (for _array_element _outactors
      (Utilities|IsValid _array_element
        (:Is%20Valid
          (bind _blackboard (Variables|/Script/AIModule.AIController|GetBlackboard _array_element)
            (:then
              (if (ScalableFloat|GetValueasBool _blackboard (Utilities|Name|MakeLiteralName "PlayerDetected"))
                (CallFunction|WinDefeat "Вас обнаружили!" (Utilities|Struct|MakeSlateColor "(R=0.500000,G=0.000000,B=0.000000,A=1.000000)" "UseColor_Specified") "/Game/StealthShooter_2/Assets/Sound/A_Defeat.A_Defeat")
                (Default|CallOnComplete false self)
                (goto _label_2 Close)))
            (:else)))))
    (Utilities|FlowControl|DelayUntilNextTick)
    (Utilities|FlowControl|Gate false :!label _label_2
      (:Exit
        (goto _label)))
    (else
      (Utilities|FlowControl|DelayUntilNextTick)
      (goto _label))))

(fn ConstructionScript
  (|CallParentFunction))