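; Survival quest actor that succeeds when the player outlasts a timer and fails, destroying itself, if the player dies first.
; A delayed gate loop refreshes the task's countdown text every second until completion, and both outcomes show a result with sound and report to the quest system.
; Success activates a message actor, which Box1 deactivates on player overlap.
; Box saves player data and opens the assigned level when the player enters at full health.
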(event OnComponentBeginOverlap(Box)
  (params (OverlappedComponent :type Primitive%20Component%20Object%20Reference) (OtherActor :type Actor%20Object%20Reference) (OtherComp :type Primitive%20Component%20Object%20Reference) (OtherBodyIndex :type Integer) (bFromSweep :type Boolean) (SweepResult :type Hit%20Result%20Structure%20%28by%20ref%29))
  (bind _asbp_player_character_stealth_shooter_2 (Utilities|Casting|CastToBP_PlayerCharacterStealthShooter_2 OtherActor))
  (if (== (Variables|/Game/StealthShooter_2/Blueprints/Core/Character/BP_BaseCharacter.BP_BaseCharacter_C|GetHealth _asbp_player_character_stealth_shooter_2) (Variables|/Game/StealthShooter_2/Blueprints/Core/Character/BP_BaseCharacter.BP_BaseCharacter_C|GetMaxHealth _asbp_player_character_stealth_shooter_2))
    (Utilities|FlowControl|Delay 1.0)
    (Default|SaveDataPlayer (Variables|/Game/StealthShooter_2/Blueprints/DataAsset/PDA_GameplayClasses.PDA_GameplayClasses_C|GetGameInstance (Variables|Default|GetGameplayClasses)))
    (Game|OpenLevel(byObjectReference) (Variables|Default|GetLevel))))

(event OnComponentBeginOverlap(Box1)
  (params (OverlappedComponent :type Primitive%20Component%20Object%20Reference) (OtherActor :type Actor%20Object%20Reference) (OtherComp :type Primitive%20Component%20Object%20Reference) (OtherBodyIndex :type Integer) (bFromSweep :type Boolean) (SweepResult :type Hit%20Result%20Structure%20%28by%20ref%29))
  (if (Actor|ActorHasTag OtherActor "Player")
    (Class|BPIActivate|Activate(Message) (Variables|Default|GetActor) false)))

(event Custom|Complete
  (CallFunction|WinDefeat "Выполнено!" (Utilities|Struct|MakeSlateColor "(R=0.000000,G=0.500000,B=0.000000,A=1.000000)" "UseColor_Specified") "/Game/StealthShooter_2/Assets/Sound/A_Win.A_Win")
  (Default|CallOnComplete true self)
  (Utilities|FlowControl|Sequence
    (:then_0
      (Utilities|FlowControl|Gate false) ; enters at Close
    )
    (:then_1
      (Class|BPIActivate|Activate(Message) (Variables|Default|GetActor) true)
      (Utilities|FlowControl|Delay 2.0)
      (CallFunction|WinDefeat " "))))

(event Custom|Defeat
  (CallFunction|WinDefeat "Провал!" (Utilities|Struct|MakeSlateColor "(R=0.500000,G=0.000000,B=0.000000,A=1.000000)" "UseColor_Specified") "/Game/StealthShooter_2/Assets/Sound/A_Defeat.A_Defeat")
  (Default|CallOnComplete false self)
  (Utilities|Time|ClearandInvalidateTimerbyHandle (Variables|Default|GetTimer))
  (Actor|DestroyActor))

(event EventStart
  (Utilities|FlowControl|Sequence
    (:then_0
      (EventDispatchers|BindEventtoOnDeath (Variables|/Game/StealthShooter_2/Blueprints/DataAsset/PDA_GameplayClasses.PDA_GameplayClasses_C|GetPlayerCharacter (Variables|Default|GetGameplayClasses)) (delegate Custom|Defeat)))
    (:then_1
      (Utilities|FlowControl|Delay 1.0)
      (CallFunction|WinDefeat))
    (:then_2
      (bind _returnvalue (Utilities|Time|SetTimerbyEvent (delegate Custom|Complete) (Variables|Default|GetTime)))
      (bind _output_get (Variables|Default|SetTimer _returnvalue))
      (Variables|/Script/UMG.TextBlock|SetText (Variables|/Game/StealthShooter_2/Widgets/WBP_TaskQuest.WBP_TaskQuest_C|GetTask (Utilities|Array|Get(acopy) (Variables|Default|GetTasks))) (Utilities|Text|FormatText "Продержаться {Time}" (Math|Float|Truncate (Utilities|Time|GetTimerRemainingTimebyHandle _output_get))) :!label _label)
      (Utilities|FlowControl|Delay 1.0)
      (Utilities|FlowControl|Gate false
        (:Exit
          (goto _label))))))

(fn ConstructionScript
  (|CallParentFunction))