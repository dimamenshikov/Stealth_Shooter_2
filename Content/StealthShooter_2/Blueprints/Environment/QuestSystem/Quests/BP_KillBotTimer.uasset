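; Timed quest to kill a set number of bots, extending a parent quest with a time limit.
; On start it sets a timer and rewrites a task line with the remaining seconds every second.
; Completion clears the timer and stops the countdown; expiry shows a defeat message, reports failure and destroys the actor.
; Gates make winning and losing mutually exclusive, so the failure's completion call does not trigger the win path.
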(event Custom|Lose
  ;[0 0 0] Квест на убийство определённого количества ботов за определённое время, вывод информации на экран
  (Utilities|FlowControl|Gate false
    (:Exit
      (Utilities|FlowControl|Sequence
        (:then_0
          (Utilities|FlowControl|Gate false) ; enters at Close
        )
        (:then_1
          (CallFunction|WinDefeat "Время вышло!" (Utilities|Struct|MakeSlateColor "(R=0.500000,G=0.000000,B=0.000000,A=1.000000)" "UseColor_Specified") "/Game/StealthShooter_2/Assets/Sound/A_Defeat.A_Defeat")
          (Default|CallOnComplete false self)
          (Actor|DestroyActor))))))

(event Custom|Win
  (params (Success :type Boolean) (Quest :type BP%20Base%20Quest%20Object%20Reference))
  ;[0 0 0] Квест на убийство определённого количества ботов за определённое время, вывод информации на экран
  (Utilities|FlowControl|Gate false
    (:Exit
      (Utilities|FlowControl|Sequence
        (:then_0
          (Utilities|Time|ClearandInvalidateTimerbyHandle (Variables|Default|GetTimer))
          (Utilities|FlowControl|Gate false) ; enters at Close
        )
        (:then_1
          (Utilities|FlowControl|Gate false) ; enters at Close
        )))))

(event EventStart
  ;[0 0 0] Квест на убийство определённого количества ботов за определённое время, вывод информации на экран
  (|CallParentFunction)
  (bind _returnvalue (Utilities|Time|SetTimerbyEvent (delegate Custom|Lose) (Variables|Default|GetTime)))
  (Variables|Default|SetTimer _returnvalue)
  (EventDispatchers|BindEventtoOnComplete (delegate Custom|Win))
  (Variables|/Script/UMG.TextBlock|SetText (Variables|/Game/StealthShooter_2/Widgets/WBP_TaskQuest.WBP_TaskQuest_C|GetTask (Utilities|Array|Get(acopy) (Variables|Default|GetTasks) 2)) (Utilities|Text|FormatText "Осталось  времени {Time}" (Math|Float|Truncate (Utilities|Time|GetTimerRemainingTimebyHandle (Variables|Default|GetTimer)))) :!label _label)
  (Utilities|FlowControl|Delay 1.0)
  (Utilities|FlowControl|Gate false
    (:Exit
      (goto _label))))

(fn ConstructionScript
  (|CallParentFunction))