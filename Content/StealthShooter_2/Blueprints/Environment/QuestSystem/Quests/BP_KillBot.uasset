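; Kill-bot quest that requires destroying a set number of spawned enemies and shows the remaining count in its task text.
; It binds to the enemy spawner and hooks each new enemy's destroyed event to count kills and refresh the text.
; Reaching the quota means success and player death means failure.
; Both outcomes share one ending that fires the completion callback, shows a colored result with sound and destroys the quest actor.
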(event Custom|SpawnNewEnemy
  (params (NewEnemy :type BP%20Enemy%20Object%20Reference))
  ;[0 0 0] Квест на убийство определённого количества ботов, вывод информации квеста на экран
  (Game|BindEventtoOnDestroyed NewEnemy (delegate Custom|EnemDead)))

(event Custom|EnemDead
  (params (DestroyedActor :type Actor%20Object%20Reference))
  (bind _quantitykillbot (Variables|Default|GetQuantityKillBot))
  ;[0 0 0] Квест на убийство определённого количества ботов, вывод информации квеста на экран
  (bind _result (Math|Integer|IncrementInt (Variables|Default|GetCountKills))
    (:%20%20
      (Variables|/Script/UMG.TextBlock|SetText (Variables|/Game/StealthShooter_2/Widgets/WBP_TaskQuest.WBP_TaskQuest_C|GetTask (Utilities|Array|Get(acopy) (Variables|Default|GetTasks) 1)) (Utilities|Text|FormatText "Убить ботов {Count}/{Quantity}" (- _quantitykillbot (Variables|Default|GetCountKills)) _quantitykillbot))
      (if (== _result (Variables|Default|GetQuantityKillBot))
        (Variables|Default|SetSuccess true)
        (Default|CallOnComplete (Variables|Default|GetSuccess) self)
        (CallFunction|WinDefeat (Utilities|String|SelectText "Выполнено!" "Вас убили!" (Variables|Default|GetSuccess)) (Utilities|Struct|MakeSlateColor (Math|Color|SelectColor "(R=0.000000,G=0.500000,B=0.000000,A=1.000000)" "(R=0.500000,G=0.000000,B=0.000000,A=1.000000)" (Variables|Default|GetSuccess)) "UseColor_Specified") (select (Variables|Default|GetSuccess) "/Game/StealthShooter_2/Assets/Sound/A_Win.A_Win" "/Game/StealthShooter_2/Assets/Sound/A_Defeat.A_Defeat"))
        (Actor|DestroyActor)))))

(event Custom|Defeat
  ;[0 0 0] Квест на убийство определённого количества ботов, вывод информации квеста на экран
  (Variables|Default|SetSuccess false)
  (Default|CallOnComplete (Variables|Default|GetSuccess) self)
  (CallFunction|WinDefeat (Utilities|String|SelectText "Выполнено!" "Вас убили!" (Variables|Default|GetSuccess)) (Utilities|Struct|MakeSlateColor (Math|Color|SelectColor "(R=0.000000,G=0.500000,B=0.000000,A=1.000000)" "(R=0.500000,G=0.000000,B=0.000000,A=1.000000)" (Variables|Default|GetSuccess)) "UseColor_Specified") (select (Variables|Default|GetSuccess) "/Game/StealthShooter_2/Assets/Sound/A_Win.A_Win" "/Game/StealthShooter_2/Assets/Sound/A_Defeat.A_Defeat"))
  (Actor|DestroyActor))

(event EventStart
  (bind _quantitykillbot (Variables|Default|GetQuantityKillBot))
  ;[0 0 0] Квест на убийство определённого количества ботов, вывод информации квеста на экран
  (Variables|/Script/UMG.TextBlock|SetText (Variables|/Game/StealthShooter_2/Widgets/WBP_TaskQuest.WBP_TaskQuest_C|GetTask (Utilities|Array|Get(acopy) (Variables|Default|GetTasks) 1)) (Utilities|Text|FormatText "Убить ботов {Count}/{Quantity}" (- _quantitykillbot (Variables|Default|GetCountKills)) _quantitykillbot))
  (EventDispatchers|BindEventtoOnSpawnNewEmeny (Variables|Default|GetSpawnEnemy) (delegate Custom|SpawnNewEnemy))
  (EventDispatchers|BindEventtoOnDeath (Variables|/Game/StealthShooter_2/Blueprints/DataAsset/PDA_GameplayClasses.PDA_GameplayClasses_C|GetPlayerCharacter (Variables|Default|GetGameplayClasses)) (delegate Custom|Defeat)))

(fn ConstructionScript
  (|CallParentFunction))