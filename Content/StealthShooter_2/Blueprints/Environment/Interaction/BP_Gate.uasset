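; BP_Gate is an environment gate that sinks when activated and rises again after a Duration delay once deactivated.
; The UpDown timeline, rate-scaled by Time, lerps the actor's Z from its start height by a scale-dependent offset.
; A Gate flow node blocks the delayed rise if the gate is reactivated meanwhile.
; A 2D sound plays during movement at the game options volume, and Open activates it on BeginPlay.
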(event EventBeginPlay
  ;[0 0 0] Установка скорости открывания ворот, создание звука
  (Variables|Default|SetStart_Z_Location (.z (Transformation|GetActorLocation)))
  (Components|Timeline|SetPlayRate (Variables|Default|GetUpDown) (/ 1.0 (Variables|Default|GetTime)))
  (if (Variables|Default|GetOpen)
    (CallFunction|Activate true))
  (bind _returnvalue (Audio|CreateSound2D "/Game/StealthShooter_2/Assets/Sound/A_Gate.A_Gate" (.volume (Variables|/Game/StealthShooter_2/Blueprints/Core/BP_GameInstance.BP_GameInstance_C|GetGameOptions (CallFunction|GameInstance))) 1.0 0.0 0 false false))
  (Variables|Default|SetGateSound _returnvalue))

(event EventActivate
  (params (Activate :type Boolean))
  (bind _returnvalue (Transformation|GetActorLocation))
  (bind _start_z_location (Variables|Default|GetStart_Z_Location))
  ;[0 0 0] Поднимание и опускание ворот при нажатии на кнопку
  (Variables|Default|SetBegin_Z_Location _start_z_location)
  (Variables|Default|SetEnd_Z_Location (+ _start_z_location (* (.z (Transformation|GetActorScale3D)) -301.0)))
  (if Activate
    (Utilities|FlowControl|Sequence
      (:then_0
        (goto _label Close))
      (:then_1
        (bind _gatesound (Variables|Default|GetGateSound)
          (:then
            (Class|AudioComponent|SetPaused _gatesound false)
            (Audio|Components|Audio|Play _gatesound 0.0)
            (bind _scalez (Timeline|UpDown Play)
              (:Update
                (Transformation|SetActorLocation (Math|Vector|MakeVector (.x _returnvalue) (.y _returnvalue) (Math|Float|Lerp (Variables|Default|GetBegin_Z_Location) (Variables|Default|GetEnd_Z_Location) _scalez)) false true))
              (:Finished
                (bind _gatesound_2 (Variables|Default|GetGateSound)
                  (:then
                    (Class|AudioComponent|SetPaused _gatesound_2 true)
                    (Audio|Components|Audio|SetVolumeMultiplier _gatesound_2 (.volume (Variables|/Game/StealthShooter_2/Blueprints/Core/BP_GameInstance.BP_GameInstance_C|GetGameOptions (CallFunction|GameInstance))) :!class /Script/Engine.AudioComponent))
                  (:else)))))
          (:else
            (Timeline|UpDown Play)))))
    (else
      (Utilities|FlowControl|Sequence
        (:then_0
          (Utilities|FlowControl|Delay (Variables|Default|GetDuration))
          (Utilities|FlowControl|Gate false :!label _label
            (:Exit
              (bind _gatesound_3 (Variables|Default|GetGateSound)
                (:then
                  (Class|AudioComponent|SetPaused _gatesound_3 false)
                  (Audio|Components|Audio|Play _gatesound_3 0.0)
                  (Timeline|UpDown Reverse))
                (:else
                  (Timeline|UpDown Reverse))))))
        (:then_1
          (goto _label Open))))))

(fn ConstructionScript)