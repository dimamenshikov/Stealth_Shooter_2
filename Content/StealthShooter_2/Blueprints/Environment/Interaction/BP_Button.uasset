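; BP_Button is an overlap-triggered button that switches a referenced actor on and off in the stealth shooter's environment.
; Entering or leaving its Box plays a click at the game options volume and runs the UpDown timeline forward or backward to move the button vertically.
; The actor receives ActivateMessage true only when the forward movement finishes, but receives false immediately when the overlap ends.
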(event OnComponentBeginOverlap(Box)
  (params (OverlappedComponent :type Primitive%20Component%20Object%20Reference) (OtherActor :type Actor%20Object%20Reference) (OtherComp :type Primitive%20Component%20Object%20Reference) (OtherBodyIndex :type Integer) (bFromSweep :type Boolean) (SweepResult :type Hit%20Result%20Structure%20%28by%20ref%29))
  ;[0 0 0] Поднимание или опускание кнопки, проигрывание звука, включение или отключение актора
  (Audio|PlaySound2D "/Game/StealthShooter_2/Assets/Sound/A_Button.A_Button" (.volume (Variables|/Game/StealthShooter_2/Blueprints/Core/BP_GameInstance.BP_GameInstance_C|GetGameOptions (CallFunction|GameInstance))) 1.0 0.0 0 0)
  (bind (_direction _locaionz) (Timeline|UpDown Play)
    (:Update
      (Transformation|SetRelativeLocation (Variables|Default|GetButton) (Math|Vector|MakeVector 0.0 0.0 _locaionz) false false))
    (:Finished
      (if (Utilities|Enum|Equal(Enum) _direction "Forward")
        (Class|BPIActivate|Activate(Message) (Variables|Default|GetActor) true)))))

(event OnComponentEndOverlap(Box)
  (params (OverlappedComponent :type Primitive%20Component%20Object%20Reference) (OtherActor :type Actor%20Object%20Reference) (OtherComp :type Primitive%20Component%20Object%20Reference) (OtherBodyIndex :type Integer))
  ;[0 0 0] Поднимание или опускание кнопки, проигрывание звука, включение или отключение актора
  (Class|BPIActivate|Activate(Message) (Variables|Default|GetActor) false)
  (Audio|PlaySound2D "/Game/StealthShooter_2/Assets/Sound/A_Button.A_Button" (.volume (Variables|/Game/StealthShooter_2/Blueprints/Core/BP_GameInstance.BP_GameInstance_C|GetGameOptions (CallFunction|GameInstance))) 1.0 0.0 0 0)
  (bind (_direction _locaionz) (Timeline|UpDown Reverse)
    (:Update
      (Transformation|SetRelativeLocation (Variables|Default|GetButton) (Math|Vector|MakeVector 0.0 0.0 _locaionz) false false))
    (:Finished
      (if (Utilities|Enum|Equal(Enum) _direction "Forward")
        (Class|BPIActivate|Activate(Message) (Variables|Default|GetActor) true)))))

(fn ConstructionScript)