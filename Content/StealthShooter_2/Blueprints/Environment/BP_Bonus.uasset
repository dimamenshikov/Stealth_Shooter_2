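; Base pickup Blueprint for player bonuses in StealthShooter_2, with Take and ActivateBonus left as stubs, so it grants nothing itself.
; When the player character overlaps the Box and Take accepts, a DoOnce hides the Bonus, plays a volume-scaled sound and calls ActivateBonus.
; After the Duration delay, the bonus reappears and the DoOnce resets, unless OneOnly is set.
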(event OnComponentBeginOverlap(Box)
  (params (OverlappedComponent :type Primitive%20Component%20Object%20Reference) (OtherActor :type Actor%20Object%20Reference) (OtherComp :type Primitive%20Component%20Object%20Reference) (OtherBodyIndex :type Integer) (bFromSweep :type Boolean) (SweepResult :type Hit%20Result%20Structure%20%28by%20ref%29))
  ;[0 0 0] Подбор предмета, проигрывание звука
  (bind _asbp_player_character_stealth_shooter_2 (Utilities|Casting|CastToBP_PlayerCharacterStealthShooter_2 OtherActor))
  (if (CallFunction|Take _asbp_player_character_stealth_shooter_2)
    (Utilities|FlowControl|DoOnce false :!label _label
      (:Completed
        (Development|SetHiddeninGame (Variables|Default|GetBonus) true false)
        (Audio|PlaySoundatLocation (Variables|Default|GetSound) (.location SweepResult) "0, 0, 0" (.volume (Variables|/Game/StealthShooter_2/Blueprints/Core/BP_GameInstance.BP_GameInstance_C|GetGameOptions (CallFunction|GameInstance))) 1.0 0.0 0 0 0 0)
        (CallFunction|ActivateBonus _asbp_player_character_stealth_shooter_2)
        (Utilities|FlowControl|Delay (Variables|Default|GetDuration))
        (if (not (Variables|Default|GetOneOnly))
          (Development|SetHiddeninGame (Variables|Default|GetBonus) false false)
          (goto _label Reset))))))

(event Custom|ActivateBonus
  (params (Player :type BP%20Player%20Character%20Stealth%20Shooter%202%20Object%20Reference))
  ;[0 0 0] Подбор предмета, проигрывание звука
)

(fn ConstructionScript)

(fn Take
  (params (Player :type BP%20Player%20Character%20Stealth%20Shooter%202%20Object%20Reference))
  (return false))