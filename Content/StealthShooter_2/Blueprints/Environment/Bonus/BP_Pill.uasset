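; BP_Pill is a health pickup bonus that heals the player.
; ActivateBonus adds a fixed amount to the player's Health, clamped to MaxHealth.
; Take allows pickup only while the player's Health is below maximum.
; The construction script just calls its parent's.
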(event EventActivateBonus
  (params (Player :type BP%20Player%20Character%20Stealth%20Shooter%202%20Object%20Reference))
  ;[0 0 0] Увеличение здоровья
  (Variables|/Game/StealthShooter_2/Blueprints/Core/Character/BP_BaseCharacter.BP_BaseCharacter_C|SetHealth Player (Math|Float|Clamp(Float) (+ (Variables|/Game/StealthShooter_2/Blueprints/Core/Character/BP_BaseCharacter.BP_BaseCharacter_C|GetHealth Player) 3e+01) 0.0 (Variables|/Game/StealthShooter_2/Blueprints/Core/Character/BP_BaseCharacter.BP_BaseCharacter_C|GetMaxHealth Player))))

(fn ConstructionScript
  (|CallParentFunction))

(fn Take
  (params (Player :type BP%20Player%20Character%20Stealth%20Shooter%202%20Object%20Reference))
  ;[0 0 0] Проверка можно ли взять аптечку
  (return (< (Variables|/Game/StealthShooter_2/Blueprints/Core/Character/BP_BaseCharacter.BP_BaseCharacter_C|GetHealth Player) (Variables|/Game/StealthShooter_2/Blueprints/Core/Character/BP_BaseCharacter.BP_BaseCharacter_C|GetMaxHealth Player))))