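; Enemy spawner that keeps a set number of BP_Enemy bots alive in a level, with an optional cap on total spawns.
; On BeginPlay it caches its spline points and hands them to each bot as a patrol route.
; Bots spawn in a delayed recursive chain at random PointSpawn actors, toggling their doors and firing a spawn dispatcher.
; Bot destruction triggers replacements; the construction script sizes the spawn-zone box.
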(event Custom|SpawnEnem
  (bind _quantityborder (Variables|Default|GetQuantityBorder))
  ;[0 0 0] Создание ботов, передача им точек их маршрута, контроль количества созданных ботов и ботов на уровне
  (bind _output_get (Variables|Default|SetRandomPoint (.OutItem (Utilities|Array|Random (Variables|Default|GetPointSpawn)))))
  (bind _returnvalue (Game|SpawnActorfromClass "/Game/StealthShooter_2/AI/Guard/BP_Enemy.BP_Enemy_C" (Math|Transform|MakeTransform (+ "0.000000,0.000000,90.000000" (.location (Transformation|GetActorTransform _output_get))) (.rotation (Transformation|GetActorTransform _output_get)) "1.000000,1.000000,1.000000") "AlwaysSpawn" "MultiplyWithRoot" 0 0))
  (Default|OpenDoor (Variables|Default|GetRandomPoint) false)
  (Default|CallOnSpawnNewEmeny _returnvalue)
  (Variables|/Game/StealthShooter_2/AI/Guard/BP_Enemy.BP_Enemy_C|SetPointPoute _returnvalue (Variables|Default|GetPoints))
  (Math|Integer|IncrementInt (Variables|Default|GetCount)
    (:%20%20
      (Math|Integer|IncrementInt (Variables|Default|GetQuantity)
        (:%20%20
          (Game|BindEventtoOnDestroyed _returnvalue (delegate Custom|EnemDead))
          (Utilities|FlowControl|Delay 1.5)
          (Default|OpenDoor (Variables|Default|GetRandomPoint) true)
          (Utilities|FlowControl|Delay 1.0)
          (if (and (< (Variables|Default|GetCount) (Variables|Default|GetQuantityEnemy)) (or (< (Variables|Default|GetQuantity) _quantityborder) (== _quantityborder 0)))
            (CallFunction|SpawnEnem)))))))

(event Custom|EnemDead
  (params (DestroyedActor :type Actor%20Object%20Reference))
  (bind _quantityborder (Variables|Default|GetQuantityBorder))
  ;[0 0 0] Создание ботов, передача им точек их маршрута, контроль количества созданных ботов и ботов на уровне
  (Math|Integer|DecrementInt (Variables|Default|GetCount)
    (:%20%20
      (if (or (< (Variables|Default|GetQuantity) _quantityborder) (== _quantityborder 0))
        (CallFunction|SpawnEnem)))))

(event EventBeginPlay
  ;[0 0 0] Получение точек маршрута ботов, запуск создания ботов
  (for _index (range 0 (- (Spline|GetNumberOfSplinePoints (Variables|/Game/StealthShooter_2/Blueprints/Environment/BP_PatrolRoute.BP_PatrolRoute_C|GetSpline (Variables|Default|GetSpline))) 1))
    (Utilities|Array|Add (Variables|Default|GetPoints) (Spline|GetLocationatSplinePoint (Variables|/Game/StealthShooter_2/Blueprints/Environment/BP_PatrolRoute.BP_PatrolRoute_C|GetSpline (Variables|Default|GetSpline)) _index "World")))
  (Utilities|FlowControl|Delay 1.0)
  (CallFunction|SpawnEnem))

(fn ConstructionScript
  (bind _box (Variables|Default|GetBox))
  (Transformation|SetRelativeLocation _box (Math|Vector|MakeVector 0.0 0.0 (.z (Variables|Default|GetSizeSpawnZone))) false false)
  (Components|Box|SetBoxExtent _box (Variables|Default|GetSizeSpawnZone) true))