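; Player controller for a stealth shooter that registers itself in GameplayClasses and maps Enhanced Input to movement, look, pause and a held controls-help overlay.
; Actions like jump, reload, sprint and crouch call the living character's ActiveAbility, with GAS tags supplying current state.
; Gates with delays make an Aim tap toggle shooting mode and a hold aim, both blocked while crouched, while holding Shoot repeats fire.
; GetAim exposes the aim input.
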(event Input|EnhancedActionEvents|EnhancedInputActionIA_Pause
  (params (ActionValue :type Boolean) (ElapsedSeconds :type Float%20%28double-precision%29) (TriggeredSeconds :type Float%20%28double-precision%29) (InputAction :type Input%20Action%20Object%20Reference :default "/Game/StealthShooter_2/Blueprints/Input/Actions/IA_Pause.IA_Pause"))
  ;[0 0 0] Пауза
  (:Started
    (Default|PauseGame (Variables|/Game/StealthShooter_2/Blueprints/DataAsset/PDA_GameplayClasses.PDA_GameplayClasses_C|GetGameMode (Variables|Default|GetGameplayClasses)) (not (Game|IsGamePaused)))))

(event Input|EnhancedActionEvents|EnhancedInputActionIA_Look
  (params (ActionValue :type Vector%202D%20Structure) (ElapsedSeconds :type Float%20%28double-precision%29) (TriggeredSeconds :type Float%20%28double-precision%29) (InputAction :type Input%20Action%20Object%20Reference :default "/Game/StealthShooter_2/Blueprints/Input/Actions/IA_Look.IA_Look"))
  ;[0 0 0] Поворот камеры игрока
  (Class|PlayerController|AddYawInput (.x ActionValue))
  (Class|PlayerController|AddPitchInput (.y ActionValue)))

(event Input|EnhancedActionEvents|EnhancedInputActionIA_Move
  (params (ActionValue :type Vector%202D%20Structure) (ElapsedSeconds :type Float%20%28double-precision%29) (TriggeredSeconds :type Float%20%28double-precision%29) (InputAction :type Input%20Action%20Object%20Reference :default "/Game/StealthShooter_2/Blueprints/Input/Actions/IA_Move.IA_Move"))
  ;[0 0 0] Движение игрока
  (bind _playercharacter (Variables|/Game/StealthShooter_2/Blueprints/DataAsset/PDA_GameplayClasses.PDA_GameplayClasses_C|GetPlayerCharacter (Variables|Default|GetGameplayClasses))
    (:then
      (if (not (Variables|/Game/StealthShooter_2/Blueprints/Core/Character/BP_BaseCharacter.BP_BaseCharacter_C|GetbDeath _playercharacter))
        (Pawn|Input|AddMovementInput _playercharacter (Math|Vector|RotateVector (Math|Conversions|ToVector(Vector2D) ActionValue) (Math|Rotator|MakeRotator 0.0 0.0 (.yaw (Pawn|GetControlRotation :!class /Script/Engine.Controller)))) 1.0 false)))
    (:else)))

(event Input|EnhancedActionEvents|EnhancedInputActionIA_Management
  (params (ActionValue :type Boolean) (ElapsedSeconds :type Float%20%28double-precision%29) (TriggeredSeconds :type Float%20%28double-precision%29) (InputAction :type Input%20Action%20Object%20Reference :default "/Game/StealthShooter_2/Blueprints/Input/Actions/IA_Management.IA_Management"))
  (bind _gameplayclasses (Variables|Default|GetGameplayClasses))
  (bind _hud (Variables|/Game/StealthShooter_2/Blueprints/DataAsset/PDA_GameplayClasses.PDA_GameplayClasses_C|GetHUD _gameplayclasses))
  (bind _interface (Default|GetInterface _hud))
  (bind _management (Variables|/Game/StealthShooter_2/Widgets/WBP_Interface.WBP_Interface_C|GetManagement _interface))
  ;[0 0 0] Показ системы управления персонажем
  (:Started
    (Widget|SetVisibility _management "Visible"))
  (:Completed
    (Widget|SetVisibility _management "Hidden")))

(event Input|EnhancedActionEvents|EnhancedInputActionIA_Jump
  (params (ActionValue :type Boolean) (ElapsedSeconds :type Float%20%28double-precision%29) (TriggeredSeconds :type Float%20%28double-precision%29) (InputAction :type Input%20Action%20Object%20Reference :default "/Game/StealthShooter_2/Blueprints/Input/Actions/IA_Jump.IA_Jump"))
  ;[0 0 0] Прыжок и перезарядка
  (:Started
    (bind _playercharacter (Variables|/Game/StealthShooter_2/Blueprints/DataAsset/PDA_GameplayClasses.PDA_GameplayClasses_C|GetPlayerCharacter (Variables|Default|GetGameplayClasses))
      (:then
        (if (not (Variables|/Game/StealthShooter_2/Blueprints/Core/Character/BP_BaseCharacter.BP_BaseCharacter_C|GetbDeath _playercharacter))
          (Default|ActiveAbility _playercharacter true "NewEnumerator4")))
      (:else))))

(event Input|EnhancedActionEvents|EnhancedInputActionIA_Sprint
  (params (ActionValue :type Boolean) (ElapsedSeconds :type Float%20%28double-precision%29) (TriggeredSeconds :type Float%20%28double-precision%29) (InputAction :type Input%20Action%20Object%20Reference :default "/Game/StealthShooter_2/Blueprints/Input/Actions/IA_Sprint.IA_Sprint"))
  (bind _gameplayclasses (Variables|Default|GetGameplayClasses))
  ;[0 0 0] Спринт
  (:Started
    (bind _playercharacter (Variables|/Game/StealthShooter_2/Blueprints/DataAsset/PDA_GameplayClasses.PDA_GameplayClasses_C|GetPlayerCharacter _gameplayclasses)
      (:then
        (if (not (Variables|/Game/StealthShooter_2/Blueprints/Core/Character/BP_BaseCharacter.BP_BaseCharacter_C|GetbDeath _playercharacter))
          (Default|ActiveAbility _playercharacter true "NewEnumerator0")))
      (:else)))
  (:Completed
    (bind _playercharacter_2 (Variables|/Game/StealthShooter_2/Blueprints/DataAsset/PDA_GameplayClasses.PDA_GameplayClasses_C|GetPlayerCharacter _gameplayclasses)
      (:then
        (if (not (Variables|/Game/StealthShooter_2/Blueprints/Core/Character/BP_BaseCharacter.BP_BaseCharacter_C|GetbDeath _playercharacter_2))
          (Default|ActiveAbility _playercharacter_2 false "NewEnumerator0")))
      (:else))))

(event Input|EnhancedActionEvents|EnhancedInputActionIA_Crouch
  (params (ActionValue :type Boolean) (ElapsedSeconds :type Float%20%28double-precision%29) (TriggeredSeconds :type Float%20%28double-precision%29) (InputAction :type Input%20Action%20Object%20Reference :default "/Game/StealthShooter_2/Blueprints/Input/Actions/IA_Crouch.IA_Crouch"))
  (bind _gameplayclasses (Variables|Default|GetGameplayClasses))
  (bind _playercharacter (Variables|/Game/StealthShooter_2/Blueprints/DataAsset/PDA_GameplayClasses.PDA_GameplayClasses_C|GetPlayerCharacter _gameplayclasses))
  (bind _abilitysystem (Variables|/Game/StealthShooter_2/Blueprints/Core/Character/BP_BaseCharacter.BP_BaseCharacter_C|GetAbilitySystem _playercharacter))
  (bind _tagcontainer (GameplayTags|GetOwnedGameplayTags _abilitysystem :!class /Script/GameplayTags.GameplayTagAssetInterface))
  (bind _returnvalue (GameplayTags|HasTag _tagcontainer "(TagName=\"Status.Character.Crouch\")"))
  ;[0 0 0] Присед
  (:Started
    (bind _playercharacter_2 (Variables|/Game/StealthShooter_2/Blueprints/DataAsset/PDA_GameplayClasses.PDA_GameplayClasses_C|GetPlayerCharacter (Variables|Default|GetGameplayClasses))
      (:then
        (if (not (Variables|/Game/StealthShooter_2/Blueprints/Core/Character/BP_BaseCharacter.BP_BaseCharacter_C|GetbDeath _playercharacter_2))
          (Default|ActiveAbility _playercharacter_2 (not _returnvalue) "NewEnumerator1")
          (Transformation|SetRelativeLocation (Variables|/Game/StealthShooter_2/Blueprints/Core/Character/BP_PlayerCharacterStealthShooter_2.BP_PlayerCharacterStealthShooter_2_C|GetScene _playercharacter_2) (Math|Vector|MakeVector 0.0 0.0 (Math|Float|SelectFloat 48.0 0.0 _returnvalue)) false false)))
      (:else))))

(event Input|EnhancedActionEvents|EnhancedInputActionIA_Aim
  (params (ActionValue :type Boolean) (ElapsedSeconds :type Float%20%28double-precision%29) (TriggeredSeconds :type Float%20%28double-precision%29) (InputAction :type Input%20Action%20Object%20Reference :default "/Game/StealthShooter_2/Blueprints/Input/Actions/IA_Aim.IA_Aim"))
  (bind _gameplayclasses (Variables|Default|GetGameplayClasses))
  (bind _gameplayclasses_2 (Variables|Default|GetGameplayClasses))
  (bind _gameplayclasses_3 (Variables|Default|GetGameplayClasses))
  (bind _playercharacter (Variables|/Game/StealthShooter_2/Blueprints/DataAsset/PDA_GameplayClasses.PDA_GameplayClasses_C|GetPlayerCharacter _gameplayclasses))
  (bind _playercharacter_2 (Variables|/Game/StealthShooter_2/Blueprints/DataAsset/PDA_GameplayClasses.PDA_GameplayClasses_C|GetPlayerCharacter _gameplayclasses_3))
  (bind _playercharacter_3 (Variables|/Game/StealthShooter_2/Blueprints/DataAsset/PDA_GameplayClasses.PDA_GameplayClasses_C|GetPlayerCharacter _gameplayclasses_2))
  (bind _abilitysystem (Variables|/Game/StealthShooter_2/Blueprints/Core/Character/BP_BaseCharacter.BP_BaseCharacter_C|GetAbilitySystem _playercharacter))
  (bind _abilitysystem_2 (Variables|/Game/StealthShooter_2/Blueprints/Core/Character/BP_BaseCharacter.BP_BaseCharacter_C|GetAbilitySystem _playercharacter_2))
  (bind _tagcontainer (GameplayTags|GetOwnedGameplayTags _abilitysystem_2 :!class /Script/GameplayTags.GameplayTagAssetInterface))
  (bind _tagcontainer_2 (GameplayTags|GetOwnedGameplayTags _abilitysystem :!class /Script/GameplayTags.GameplayTagAssetInterface))
  ;[0 0 0] Режим стрельбы
  (:Started
    (Utilities|FlowControl|Sequence
      (:then_0
        (goto _label Open))
      (:then_1
        (Utilities|FlowControl|Delay 0.25)
        (Utilities|FlowControl|Gate true :!label _label
          (:Exit
            (bind _playercharacter_4 (Variables|/Game/StealthShooter_2/Blueprints/DataAsset/PDA_GameplayClasses.PDA_GameplayClasses_C|GetPlayerCharacter (Variables|Default|GetGameplayClasses))
              (:then
                (if (and (not (GameplayTags|HasTag _tagcontainer_2 "(TagName=\"Status.Character.Crouch\")")) (not (Variables|/Game/StealthShooter_2/Blueprints/Core/Character/BP_BaseCharacter.BP_BaseCharacter_C|GetbDeath _playercharacter_4)))
                  (if (GameplayTags|HasTag _tagcontainer_2 "(TagName=\"Status.Character.ModeShoot\")")
                    _
                    (else
                      (Default|ModeShoot _playercharacter_4 true)
                      (Utilities|FlowControl|Sequence
                        (:then_0
                          (goto _label_2 Open))
                        (:then_1
                          (Utilities|FlowControl|Delay 1.2)
                          (Utilities|FlowControl|Gate true :!label _label_2
                            (:Exit
                              _))))))
                  (Default|ActiveAbility (Variables|/Game/StealthShooter_2/Blueprints/DataAsset/PDA_GameplayClasses.PDA_GameplayClasses_C|GetPlayerCharacter (Variables|Default|GetGameplayClasses)) true "NewEnumerator3")))
              (:else)))))))
  (:Completed
    (Utilities|FlowControl|Sequence
      (:then_0
        (goto _label Close))
      (:then_1
        (goto _label_2 Close))
      (:then_2
        (bind _playercharacter_5 (Variables|/Game/StealthShooter_2/Blueprints/DataAsset/PDA_GameplayClasses.PDA_GameplayClasses_C|GetPlayerCharacter _gameplayclasses_3)
          (:then
            (if (and (not (Variables|/Game/StealthShooter_2/Blueprints/Core/Character/BP_BaseCharacter.BP_BaseCharacter_C|GetbDeath _playercharacter_5)) (not (GameplayTags|HasTag _tagcontainer "(TagName=\"Status.Character.Crouch\")")))
              (if (GameplayTags|HasTag _tagcontainer "(TagName=\"Status.Character.ModeShoot\")")
                (if (GameplayTags|HasTag (GameplayTags|GetOwnedGameplayTags (Variables|/Game/StealthShooter_2/Blueprints/Core/Character/BP_BaseCharacter.BP_BaseCharacter_C|GetAbilitySystem (Variables|/Game/StealthShooter_2/Blueprints/DataAsset/PDA_GameplayClasses.PDA_GameplayClasses_C|GetPlayerCharacter (Variables|Default|GetGameplayClasses))) :!class /Script/GameplayTags.GameplayTagAssetInterface) "(TagName=\"Status.Character.Aim\")")
                  (Default|ActiveAbility _playercharacter_3 false "NewEnumerator3")
                  (else
                    (Default|ModeShoot _playercharacter_3 false)))
                (else
                  (Default|ModeShoot (Variables|/Game/StealthShooter_2/Blueprints/DataAsset/PDA_GameplayClasses.PDA_GameplayClasses_C|GetPlayerCharacter (Variables|Default|GetGameplayClasses)) true)))))
          (:else))))))

(event Input|EnhancedActionEvents|EnhancedInputActionIA_Shoot
  (params (ActionValue :type Boolean) (ElapsedSeconds :type Float%20%28double-precision%29) (TriggeredSeconds :type Float%20%28double-precision%29) (InputAction :type Input%20Action%20Object%20Reference :default "/Game/StealthShooter_2/Blueprints/Input/Actions/IA_Shoot.IA_Shoot"))
  ;[0 0 0] Стрельба
  (:Started
    (Utilities|FlowControl|Sequence
      (:then_0
        (goto _label Open))
      (:then_1
        (Utilities|FlowControl|Gate true :!label _label
          (:Exit
            (bind _playercharacter (Variables|/Game/StealthShooter_2/Blueprints/DataAsset/PDA_GameplayClasses.PDA_GameplayClasses_C|GetPlayerCharacter (Variables|Default|GetGameplayClasses))
              (:then
                (if (not (Variables|/Game/StealthShooter_2/Blueprints/Core/Character/BP_BaseCharacter.BP_BaseCharacter_C|GetbDeath _playercharacter))
                  (Default|ActiveAbility _playercharacter true "NewEnumerator2")
                  (Utilities|FlowControl|Delay 0.1)
                  (Utilities|FlowControl|Sequence
                    (:then_0
                      (goto _label)))))
              (:else)))))))
  (:Completed
    (goto _label Close)))

(event Input|EnhancedActionEvents|EnhancedInputActionIA_Reload
  (params (ActionValue :type Boolean) (ElapsedSeconds :type Float%20%28double-precision%29) (TriggeredSeconds :type Float%20%28double-precision%29) (InputAction :type Input%20Action%20Object%20Reference :default "/Game/StealthShooter_2/Blueprints/Input/Actions/IA_Reload.IA_Reload"))
  ;[0 0 0] Прыжок и перезарядка
  (:Started
    (bind _playercharacter (Variables|/Game/StealthShooter_2/Blueprints/DataAsset/PDA_GameplayClasses.PDA_GameplayClasses_C|GetPlayerCharacter (Variables|Default|GetGameplayClasses))
      (:then
        (if (not (Variables|/Game/StealthShooter_2/Blueprints/Core/Character/BP_BaseCharacter.BP_BaseCharacter_C|GetbDeath _playercharacter))
          (Default|ActiveAbility _playercharacter true "NewEnumerator5")))
      (:else))))

(event EventBeginPlay
  ;[0 0 0] Запись своей ссылки в GameplayClasses, установка системы управления
  (|CallParentFunction)
  (Variables|/Game/StealthShooter_2/Blueprints/DataAsset/PDA_GameplayClasses.PDA_GameplayClasses_C|SetPlayerController (Variables|Default|GetGameplayClasses) self)
  (Input|AddMappingContext (PlayerController|LocalPlayerSubsystems|GetEnhancedInputLocalPlayerSubsystem) "/Game/StealthShooter_2/Blueprints/Input/IMC_Management.IMC_Management" 0 "(bIgnoreAllPressedKeysUntilRelease=True,bForceImmediately=False,bNotifyUserSettings=False)")
  (Input|SetInputModeGameOnly self false))

(fn ConstructionScript)

(fn GetAim
  ;[0 0 0] Получение информации о зажатии правой кнопки мыши
  (return (Input|EnhancedActionValues|GetIA_Aim)))