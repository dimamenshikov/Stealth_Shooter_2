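; Game mode for a stealth shooter that runs level start, pause, win/defeat and the applying of game options.
; It registers itself in GameplayClasses and binds to the GameInstance start event to show the main menu or gameplay interface with matching music.
; Player defeat feeds EndGame, which after a delay pauses and shows the end screen with a result sound.
; Options set scalability and music volume, then are stored in the GameInstance.
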(event Custom|EndGame
  (params (Win :type Boolean))
  ;[0 0 0] Конец игры
  (Variables|Default|SetbWin Win)
  (Utilities|FlowControl|Delay 2.0)
  (Game|SetGamePaused true)
  (Audio|PlaySound2D (select (Variables|Default|GetbWin) "/Game/StealthShooter_2/Assets/Sound/A_Win.A_Win" "/Game/StealthShooter_2/Assets/Sound/A_Defeat.A_Defeat") (.volume (Variables|/Game/StealthShooter_2/Blueprints/Core/BP_GameInstance.BP_GameInstance_C|GetGameOptions (Variables|/Game/StealthShooter_2/Blueprints/DataAsset/PDA_GameplayClasses.PDA_GameplayClasses_C|GetGameInstance (Variables|Default|GetGameplayClasses)))) 1.0 0.0 0 0)
  (Default|ShowWidget (Variables|/Game/StealthShooter_2/Blueprints/DataAsset/PDA_GameplayClasses.PDA_GameplayClasses_C|GetHUD (Variables|Default|GetGameplayClasses)) "NewEnumerator1" true "/Game/StealthShooter_2/Widgets/WBP_EndGame.WBP_EndGame_C"))

(event Custom|StartGame
  (bind _gameplayclasses (Variables|Default|GetGameplayClasses))
  (bind _hud (Variables|/Game/StealthShooter_2/Blueprints/DataAsset/PDA_GameplayClasses.PDA_GameplayClasses_C|GetHUD _gameplayclasses))
  (bind _gameinstance (Variables|/Game/StealthShooter_2/Blueprints/DataAsset/PDA_GameplayClasses.PDA_GameplayClasses_C|GetGameInstance _gameplayclasses))
  (bind _gameoptions (Variables|/Game/StealthShooter_2/Blueprints/Core/BP_GameInstance.BP_GameInstance_C|GetGameOptions _gameinstance))
  ;[0 0 0] Начало уровня, показ виджета, проигрывание музыки
  (EventDispatchers|BindEventtoOnDefeat (Variables|/Game/StealthShooter_2/Blueprints/DataAsset/PDA_GameplayClasses.PDA_GameplayClasses_C|GetPlayerCharacter (Variables|Default|GetGameplayClasses)) (delegate Custom|Defeat))
  (bind _returnvalue (Game|GetCurrentLevelName true))
  (if (Utilities|Enum|Equal(Enum) _returnvalue "MainMenu")
    (Default|ShowWidget _hud "NewEnumerator1" true "/Game/StealthShooter_2/Widgets/WBP_MainMenu.WBP_MainMenu_C")
    (Actor|DestroyActor (Game|GetPlayerCharacter 0))
    (bind _returnvalue_2 (Audio|CreateSound2D "/Game/StealthShooter_2/Assets/Sound/A_MainMenuMusic.A_MainMenuMusic" (.volume _gameoptions) 1.0 0.0 0))
    (bind _output_get (Variables|Default|SetMainMenuMusic _returnvalue_2))
    (Audio|Components|Audio|Play _output_get 0.0)
    (else
      (Default|ShowWidget _hud "NewEnumerator0" true "/Game/StealthShooter_2/Widgets/WBP_Interface.WBP_Interface_C")
      (bind _returnvalue_3 (Audio|CreateSound2D "/Game/StealthShooter_2/Assets/Sound/A_LevelMusic.A_LevelMusic" (.volume _gameoptions) 1.0 0.0 0))
      (bind _output_get_2 (Variables|Default|SetLevelMusic _returnvalue_3))
      (Audio|Components|Audio|Play _output_get_2 0.0))))

(event Custom|Defeat
  ;[0 0 0] Начало уровня, показ виджета, проигрывание музыки
  (CallFunction|EndGame false))

(event EventBeginPlay
  (bind _gameplayclasses (Variables|Default|GetGameplayClasses))
  ;[0 0 0] Запись своей ссылки и подписка на диспатчер начало уровня
  (Variables|/Game/StealthShooter_2/Blueprints/DataAsset/PDA_GameplayClasses.PDA_GameplayClasses_C|SetGameMode _gameplayclasses self)
  (EventDispatchers|BindEventtoOnStartGame (Variables|/Game/StealthShooter_2/Blueprints/DataAsset/PDA_GameplayClasses.PDA_GameplayClasses_C|GetGameInstance _gameplayclasses) (EventDispatchers|CreateEvent :!event Custom|StartGame)))

(fn ConstructionScript)

(fn PauseGame
  (params (Pause :type Boolean))
  ;[0 0 0] Пауза
  (Game|SetGamePaused Pause)
  (Default|ShowWidget (Variables|/Game/StealthShooter_2/Blueprints/DataAsset/PDA_GameplayClasses.PDA_GameplayClasses_C|GetHUD (Variables|Default|GetGameplayClasses)) (select Pause "NewEnumerator2" "NewEnumerator0") Pause "/Game/StealthShooter_2/Widgets/WBP_PauseMenu.WBP_PauseMenu_C")
  (return))

(fn ApplyGameOptions
  (params (GameOption :type S%20Game%20Options%20Structure))
  ;[0 0 0] Применение настроек игры
  (bind _returnvalue (Settings|GetGameUserSettings))
  (Class|GameUserSettings|SetOverallScalabilityLevel _returnvalue (.graphics GameOption))
  (Class|GameUserSettings|ApplySettings _returnvalue true)
  (bind _mainmenumusic (Variables|Default|GetMainMenuMusic)
    (:then
      (Audio|Components|Audio|SetVolumeMultiplier _mainmenumusic (.volume GameOption) :!class /Script/Engine.AudioComponent))
    (:else
      _))
  (bind _levelmusic (Variables|Default|GetLevelMusic)
    (:then
      (Audio|Components|Audio|SetVolumeMultiplier _levelmusic (.volume GameOption) :!class /Script/Engine.AudioComponent))
    (:else
      _))
  (Variables|/Game/StealthShooter_2/Blueprints/Core/BP_GameInstance.BP_GameInstance_C|SetGameOptions (Variables|/Game/StealthShooter_2/Blueprints/DataAsset/PDA_GameplayClasses.PDA_GameplayClasses_C|GetGameInstance (Variables|Default|GetGameplayClasses)) (Utilities|Struct|MakeS_GameOptions (.graphics GameOption) (.volume GameOption)))
  (return))