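; BP_BaseCharacter is the base character of the stealth shooter, handling abilities, health, damage and ragdoll.
; BeginPlay grants mapped abilities with key index as InputID, which ActiveAbility presses or releases.
; Damage reduces health, triggering death at zero or otherwise alerting an undetecting enemy AI to the player's location.
; Bone impulses briefly simulate physics for hit reactions, then restore the mesh with pain effects, or push the body when dead.
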(event Custom|Death
  ;[0 0 0] Урон персонажу, отнимание здоровья, жизни
)

(event Custom|Ragdoll
  (params (bRagdoll :type Boolean))
  (bind _mesh (Variables|Character|GetMesh))
  (bind _capsulecomponent (Variables|Collision|GetCapsuleComponent))
  ;[0 0 0] Включение/отключение ragdoll
  (bind _output_get (Variables|Default|SetbDeath bRagdoll))
  (if _output_get
    (Physics|SetSimulatePhysics _mesh true)
    (Collision|SetCollisionEnabled _capsulecomponent "NoCollision")
    (else
      (Physics|SetSimulatePhysics _mesh false)
      (Transformation|SetRelativeTransform (Variables|Character|GetMesh) (Math|Transform|MakeTransform "0.000000,0.000000,-90.000000" "0.000000,-90.000000,0.000000" "1.000000,1.000000,1.000000") false false)
      (Collision|SetCollisionEnabled _capsulecomponent "QueryAndPhysics"))))

(event Custom|AddImpusleBone
  (params (impulse :type Vector))
  (bind _returnvalue (Transformation|GetActorLocation))
  (bind _mesh (Variables|Character|GetMesh))
  ;[0 0 0] Добавление импульса персонажу
  (Variables|Default|SetLocalTransformBone (Transformation|GetRelativeTransform (Variables|Character|GetMesh)))
  (Utilities|FlowControl|Delay 0.1)
  (Class|SkeletalMeshComponent|SetAllBodiesBelowSimulatePhysics (Variables|Character|GetMesh) (Utilities|Name|MakeLiteralName "spine_01") true true)
  (Physics|AddImpulse (Variables|Character|GetMesh) impulse "head" false)
  (Utilities|FlowControl|Delay 0.05)
  (if (Variables|Default|GetbDeath)
    (Physics|AddImpulse (Variables|Character|GetMesh) (* impulse 1.2) "None" true)
    (else
      (Physics|SetSimulatePhysics _mesh false)
      (Transformation|SetRelativeTransform _mesh (Variables|Default|GetLocalTransformBone) false true)
      (Audio|PlaySoundatLocation "/Game/StealthShooter_2/Assets/Sound/A_Pain.A_Pain" _returnvalue "0, 0, 0" (.volume (Variables|/Game/StealthShooter_2/Blueprints/Core/BP_GameInstance.BP_GameInstance_C|GetGameOptions (Variables|/Game/StealthShooter_2/Blueprints/DataAsset/PDA_GameplayClasses.PDA_GameplayClasses_C|GetGameInstance (Variables|Default|GetGameplayClasses)))) 1.0 0.0 0 0 0 0)
      (Effects|SpawnEmitteratLocation "/Game/StealthShooter_2/Assets/Effect/Blood/P_Blood.P_Blood" _returnvalue (Math|Rotator|Delta(Rotator) (Math|Rotator|FindLookatRotation _returnvalue (+ _returnvalue impulse)) "90.000000,0.000000,0.000000")))))

(event EventBeginPlay
  (bind _abilities (Variables|Default|GetAbilities))
  ;[0 0 0] Добавление способностей к персонажу
  (bind _keys (Utilities|Map|Keys _abilities))
  (for (_array_element _array_index) _keys
    (GameplayAbilities|GiveAbility (Variables|Default|GetAbilitySystem) (.Value (Utilities|Map|Find _abilities _array_element)) 0 _array_index)))

(event Game|Damage|EventAnyDamage
  (params (Damage :type Float%20%28single-precision%29) (DamageType :type Damage%20Type%20Object%20Reference) (InstigatedBy :type Controller%20Object%20Reference) (DamageCauser :type Actor%20Object%20Reference))
  (bind _returnvalue (Game|GetPlayerCharacter 0))
  (bind _returnvalue_2 (Utilities|Name|MakeLiteralName "PlayerDetected"))
  (bind _returnvalue_3 (Transformation|GetActorLocation _returnvalue))
  ;[0 0 0] Урон персонажу, отнимание здоровья, жизни
  (bind _output_get (Variables|Default|SetHealth (Math|Float|Clamp(Float) (- (Variables|Default|GetHealth) Damage) 0.0 (Variables|Default|GetMaxHealth))))
  (if (== _output_get 0.0)
    (Audio|PlaySoundatLocation "/Game/StealthShooter_2/Assets/Sound/A_Death.A_Death" (Transformation|GetActorLocation) "0, 0, 0" (.volume (Variables|/Game/StealthShooter_2/Blueprints/Core/BP_GameInstance.BP_GameInstance_C|GetGameOptions (Variables|/Game/StealthShooter_2/Blueprints/DataAsset/PDA_GameplayClasses.PDA_GameplayClasses_C|GetGameInstance (Variables|Default|GetGameplayClasses)))) 1.0 0.0 0 0 0 0)
    (Default|CallOnDeath)
    (CallFunction|Death)
    (else
      (bind _asaic_enemy (Utilities|Casting|CastToAIC_Enemy (AI|GetAIController self)))
      (if (not (ScalableFloat|GetValueasBool (Variables|/Script/AIModule.AIController|GetBlackboard _asaic_enemy) _returnvalue_2))
        (AI|Components|Blackboard|SetValueasBool (Variables|/Script/AIModule.AIController|GetBlackboard _asaic_enemy) _returnvalue_2 true)
        (AI|Components|Blackboard|SetValueasVector (Variables|/Script/AIModule.AIController|GetBlackboard _asaic_enemy) (Utilities|Name|MakeLiteralName "TargetLocation") _returnvalue_3)
        (AI|Components|Blackboard|SetValueasVector (Variables|/Script/AIModule.AIController|GetBlackboard _asaic_enemy) (Utilities|Name|MakeLiteralName "LastSeenLocation") _returnvalue_3)))))

(fn ConstructionScript)

(fn ActiveAbility
  (params (Activate :type Boolean) (ActiveAbility :type E_Abilities%20Enum :default "NewEnumerator6"))
  (bind _abilitysystem (Variables|Default|GetAbilitySystem))
  ;[0 0 0] Активация/деактивация способности
  (bind _keys (Utilities|Map|Keys (Variables|Default|GetAbilities)))
  (if Activate
    (Class|AbilitySystemComponent|PressInputID _abilitysystem (Utilities|Array|FindItem _keys ActiveAbility))
    (else
      (Class|AbilitySystemComponent|ReleaseInputID _abilitysystem (Utilities|Array|FindItem _keys ActiveAbility)))))