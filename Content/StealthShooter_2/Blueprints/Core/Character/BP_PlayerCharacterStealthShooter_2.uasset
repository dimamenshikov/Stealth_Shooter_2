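; Player character Blueprint for the stealth shooter, registering itself in GameplayClasses and loading its stats from the GameInstance on BeginPlay.
; Death enables ragdoll, decrements lives and signals defeat at zero, while FocusCamera switches the spring arm between close and far views.
; ModeShoot plays the equip montage forward or reversed, using notifies with Gate and DoOnce to move the rifle between back and hand, blend it via timeline and toggle abilities.
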(event Custom|ModeShoot
  (params (ModeShoot :type Boolean))
  (bind _rifle (Variables|Default|GetRifle))
  (bind _rifle_2 (Variables|Default|GetRifle))
  ;[0 0 0] Режим стрельбы
  (if ModeShoot
    (if (not (AI|Components|NavMovement|IsFalling (Variables|Character|GetCharacterMovement)))
      (Utilities|FlowControl|Sequence
        (:then_0
          (goto _label Open))
        (:then_1
          (Animation|Montage|PlayMontage (Variables|Character|GetMesh) "/Game/StealthShooter_2/Animations/MannyASP/AM_Equip_Rifle_Montage.AM_Equip_Rifle_Montage"
            (:OnNotifyBegin
              (Utilities|FlowControl|Gate true :!label _label
                (:Exit
                  (Utilities|FlowControl|Sequence
                    (:then_0
                      (Utilities|FlowControl|FlipFlop
                        (:A
                          (Transformation|AttachComponentToComponent _rifle_2 (Variables|Character|GetMesh) "hand_r" "KeepRelative" "KeepRelative" "KeepRelative" true)
                          (Transformation|SetRelativeTransform _rifle_2 (Math|Transform|MakeTransform "-11.590565,0.460342,4.436145" "3.986043,90.219046,-119.779275" "1.000000,1.000000,1.000000") false false)
                          (Audio|Components|Audio|Play (Variables|Default|GetDrawWeapon)))
                        (:B
                          (CallFunction|ActiveAbility true "NewEnumerator6"))))
                    (:then_1
                      (goto _label_2 Reset))))))))))
    (else
      (Utilities|FlowControl|Sequence
        (:then_0
          (goto _label Close))
        (:then_1
          (Animation|Montage|PlayMontage (Variables|Character|GetMesh) "/Game/StealthShooter_2/Animations/MannyASP/AM_Equip_Rifle_Montage.AM_Equip_Rifle_Montage" -1.0 1.13
            (:then
              (CallFunction|ActiveAbility false "NewEnumerator6")
              (if (GameplayTags|HasTag (GameplayTags|GetOwnedGameplayTags (Variables|Default|GetAbilitySystem) :!class /Script/GameplayTags.GameplayTagAssetInterface) "(TagName=\"Status.Character.Crouch\")")
                (CallFunction|ActiveAbility false "NewEnumerator1")
                (Transformation|SetRelativeLocation (Variables|Default|GetSpringArm) "0.000000,50.000000,40.000000" false false)))
            (:OnNotifyBegin
              (Utilities|FlowControl|DoOnce true :!label _label_2
                (:Completed
                  (Utilities|String|Reverse (Variables|Default|GetDrawWeapon))
                  (Utilities|FlowControl|Delay 0.5)
                  (Transformation|AttachComponentToComponent _rifle (Variables|Character|GetMesh) "spine_03" "KeepRelative" "KeepRelative" "KeepRelative" true)
                  (Transformation|SetRelativeTransform _rifle (Math|Transform|MakeTransform "0.032848,-15.515569,3.087912" "8.576010,-90.447712,36.101486" "1.000000,1.000000,1.000000") false false))))))))))

(event Custom|FocusCamera
  (params (FocusCamera :type Boolean))
  (bind _springarm (Variables|Default|GetSpringArm))
  ;[0 0 0] Приближение/отдаление камеры к персонажу
  (Variables|/Script/Engine.SpringArmComponent|SetSocketOffset _springarm (Math|Vector|SelectVector "0.000000,40.000000,60.000000" "0.000000,100.000000,60.000000" FocusCamera))
  (Variables|/Script/Engine.SpringArmComponent|SetTargetArmLength _springarm (Math|Float|SelectFloat 3e+01 3e+02 FocusCamera)))

(event EventBeginPlay
  (bind _gameplayclasses (Variables|Default|GetGameplayClasses))
  (bind _gameinstance (Variables|/Game/StealthShooter_2/Blueprints/DataAsset/PDA_GameplayClasses.PDA_GameplayClasses_C|GetGameInstance _gameplayclasses))
  ;[0 0 0] Запись своей ссылки в GameplayClasses, вызов диспатчера начала уровня, запись характеристик из GameInstance
  (|CallParentFunction)
  (Variables|/Game/StealthShooter_2/Blueprints/DataAsset/PDA_GameplayClasses.PDA_GameplayClasses_C|SetPlayerCharacter _gameplayclasses self)
  (Default|CallOnStartGame _gameinstance)
  (Variables|Default|SetLife (Variables|/Game/StealthShooter_2/Blueprints/Core/BP_GameInstance.BP_GameInstance_C|GetPlayerLife _gameinstance))
  (Variables|Default|SetPatronsInEquipment (Variables|/Game/StealthShooter_2/Blueprints/Core/BP_GameInstance.BP_GameInstance_C|GetPlayerPatronsInEquipment _gameinstance))
  (Variables|Default|SetPatronsInShop (Variables|/Game/StealthShooter_2/Blueprints/Core/BP_GameInstance.BP_GameInstance_C|GetPlayerPatronsInShop _gameinstance))
  (Variables|Default|SetHealth (Variables|/Game/StealthShooter_2/Blueprints/Core/BP_GameInstance.BP_GameInstance_C|GetPlayerHealth _gameinstance)))

(event EventDeath
  ;[0 0 0] Смерть персонажа, включение Ragdoll, уменьшение жизней, поражение или восстановление
  (|CallParentFunction)
  (CallFunction|Ragdoll true)
  (bind _result (Math|Integer|DecrementInt (Variables|Default|GetLife))
    (:%20%20
      (if (== _result 0)
        (Default|CallOnDefeat)))))

(fn ConstructionScript
  (|CallParentFunction))