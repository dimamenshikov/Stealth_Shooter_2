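; HUD Blueprint for StealthShooter_2 that manages screen widgets and player input mode, registering itself in GameplayClasses on BeginPlay.
; ShowWidget sets game, UI or combined input with matching cursor visibility, then adds or removes the requested widget.
; Widgets are created on first show and cached in a map keyed by class for reuse.
; GetInterface returns the cached WBP_Interface instance from that map.
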(event EventBeginPlay
  ;[0 0 0] Запись своей ссылки в GameplayClasses
  (Variables|/Game/StealthShooter_2/Blueprints/DataAsset/PDA_GameplayClasses.PDA_GameplayClasses_C|SetHUD (Variables|Default|GetGameplayClasses) self))

(fn ConstructionScript)

(fn ShowWidget
  (params (InputGame :type E_InputGame%20Enum :default "NewEnumerator0") (Show :type Boolean) (Widget :type User%20Widget%20Class%20Reference))
  (bind _returnvalue (Game|GetPlayerController 0))
  (bind _widgets (Variables|Default|GetWidgets))
  (bind (_value _returnvalue_2) (Utilities|Map|Find _widgets Widget))
  ;[0 0 0] Показ виджета и установка режима ввода контроллера
  (switch Utilities|FlowControl|Switch|SwitchonE_InputGame InputGame
    (:NewEnumerator0
      (Input|SetInputModeGameOnly _returnvalue true)
      (Variables|/Script/Engine.PlayerController|SetbShowMouseCursor _returnvalue false))
    (:NewEnumerator1
      (Input|SetInputModeUIOnly _returnvalue 0 "DoNotLock" true)
      (Variables|/Script/Engine.PlayerController|SetbShowMouseCursor _returnvalue true :!label _label))
    (:NewEnumerator2
      (Input|SetInputModeGameandUI _returnvalue 0 "DoNotLock" true true)
      (goto _label)))
  (if Show
    (if _returnvalue_2
      _
      (else
        (bind _returnvalue_3 (UserInterface|CreateWidget Widget))
        (Utilities|Map|Add (Variables|Default|GetWidgets) Widget _returnvalue_3)))
    (UserInterface|Viewport|AddtoViewport _value 0)
    (return)
    (elif _returnvalue_2
      (Widget|RemovefromParent _value)
      (return))))

(fn GetInterface
  ;[0 0 0] Получение ссылки на интерфейс
  (bind _aswbp_interface (Utilities|Casting|CastToWBP_Interface (.Value (Utilities|Map|Find (Variables|Default|GetWidgets) "/Game/StealthShooter_2/Widgets/WBP_Interface.WBP_Interface_C"))))
  (return _aswbp_interface))